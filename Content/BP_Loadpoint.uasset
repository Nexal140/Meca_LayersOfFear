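; Trigger actor that swaps World Partition runtime data layers as the first-person character passes through it.
; When the character exits the Box, it flags the overlap and sets its target Layer to Loaded.
; Tick polls until that layer's effective state is Loaded, then activates it and unloads every layer in LayerToUnload.
; The overlap flag is never reset, so polling stays armed after the first exit.
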(event OnComponentEndOverlap(Box)
  (params (OverlappedComponent :type Primitive%20Component%20Object%20Reference) (OtherActor :type Actor%20Object%20Reference) (OtherComp :type Primitive%20Component%20Object%20Reference) (OtherBodyIndex :type Integer))
  (Utilities|Casting|CastToBP_FirstPersonCharacter OtherActor)
  (Variables|Default|SetOverlapped? true)
  (DataLayers|SetDataLayerRuntimeState (WorldSubsystems|GetDataLayerSubsystem) (Variables|Default|GetLayer) "Loaded" false :!class /Script/Engine.DataLayerSubsystem))

(event EventTick
  (params (DeltaSeconds :type Float%20%28single-precision%29))
  (bind _returnvalue (WorldSubsystems|GetDataLayerSubsystem))
  (if (Math|Boolean|ANDBoolean (Variables|Default|GetOverlapped?) (Utilities|Enum|Equal(Enum) (Class|DataLayerSubsystem|GetDataLayerEffectiveRuntimeState (WorldSubsystems|GetDataLayerSubsystem) (Variables|Default|GetLayer)) "Loaded") (Class|KismetSystemLibrary|MakeLiteralBool true))
    (DataLayers|SetDataLayerRuntimeState _returnvalue (Variables|Default|GetLayer) "Activated" false :!class /Script/Engine.DataLayerSubsystem)
    (for _array_element (Variables|Default|GetLayerToUnload)
      (DataLayers|SetDataLayerRuntimeState _returnvalue _array_element "Unloaded" false :!class /Script/Engine.DataLayerSubsystem))))

(event EventBeginPlay)

(fn ConstructionScript)